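; BP_ELCharacter is a character Blueprint that layers game-state setup, look replication hooks and spectator handoff over its parent class.
; On BeginPlay it copies the health and stamina on-kill values from BP_ELGameState before running parent logic, which is skipped if the cast fails.
; Replicated look-up and turn events forward their values as absolute inputs.
; On destruction it unpossesses the controller and handles spectating.
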(event `self.ReceiveBeginPlay`
  (bind _asbp_elgame_state (cast `/Game/Mordhau/Maps/Endless/GameModeBlueprints/BP_ELGameState` (`GameplayStatics.GetGameState`)))
  (set `self.HealthOnKill` (`/Game/Mordhau/Maps/Endless/GameModeBlueprints/BP_ELGameState.HealthOnKill` _asbp_elgame_state))
  (set `self.StaminaOnKill` (`/Game/Mordhau/Maps/Endless/GameModeBlueprints/BP_ELGameState.StaminaOnKill` _asbp_elgame_state))
  (`parent.ReceiveBeginPlay`))

(event `RepicatedLookUp`
  (params (NewParam :type "Float (double-precision)"))
  (`self.LookUp` NewParam true))

(event `ReplicatedTurn`
  (params (NewParam :type "Float (double-precision)"))
  (`self.Turn` NewParam true))

(event `self.ReceiveDestroyed`
  (`MordhauUtilityLibrary.UnpossessCharacterAndHandleSpectating` (`self.GetController`))
  (`parent.ReceiveDestroyed`))

(fn `UserConstructionScript`
  (`parent.UserConstructionScript`))
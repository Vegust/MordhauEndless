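; Game state for an endless Mordhau mode with block building, storing placed cubes in CubeGrid.
; Server events place, remove, clear, save and reload cubes, rebuilding from grid coordinates at 240-unit spacing, with a busy flag blocking overlapping edits.
; It also holds changeable health, stamina and AFK rules, fakes an endless scoreboard timer, and offsets suicide penalties.
; An optional config-read kill limit ends the match through BP_ELGameMode.
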(event `AppendToGrid`
  (params (Block :type "/Game/Mordhau/Maps/Endless/CreatorsStuff/BlockInfo Structure"))
  (`KismetArrayLibrary.Array_Add` (`self.CubeGrid`) Block))

(event `ServerLoadSaveFile`
  (params (SavedGrid :type "Array of /Game/Mordhau/Maps/Endless/CreatorsStuff/BlockInfo Structure"))
  (if (not (`self.beasy`))
    (set `self.CubeGrid` SavedGrid)
    (`self.ServerReloadGrid`)))

(event `ServerInitiateBlockInfoSend`
  (params (Player :type "/Game/Mordhau/Maps/Endless/GameModeBlueprints/BP_ELController Object Reference"))
  (`/Game/Mordhau/Maps/Endless/GameModeBlueprints/BP_ELController.GetBlockInfo` Player (`KismetArrayLibrary.Array_Length` (`self.CubeGrid`))))

(event `ServerInniciateSaveOnClient`
  (params (player :type "/Game/Mordhau/Maps/Endless/GameModeBlueprints/BP_ELController Object Reference") (SaveName :type String))
  (`/Game/Mordhau/Maps/Endless/GameModeBlueprints/BP_ELController.SaveGame` player (`self.CubeGrid`) SaveName))

(event `ServerClearGrid`
  (if (not (`self.beasy`))
    (set `self.beasy` true)
    (bind _outactors (`GameplayStatics.GetAllActorsOfClass` "/Game/Mordhau/Maps/Endless/CreatorsStuff/PlacebleCube.PlacebleCube_C"))
    (for _array_element _outactors
      (`self.K2_DestroyActor` _array_element))
    (`KismetArrayLibrary.Array_Clear` (`self.CubeGrid`))
    (set `self.beasy` false)))

(event `ServerReloadGrid`
  (if (not (`self.beasy`))
    (set `self.beasy` true)
    (bind _outactors (`GameplayStatics.GetAllActorsOfClass` "/Game/Mordhau/Maps/Endless/CreatorsStuff/PlacebleCube.PlacebleCube_C"))
    (for _array_element _outactors
      (`self.K2_DestroyActor` _array_element))
    (for _array_element_2 (`self.CubeGrid`)
      (`|SpawnActorFromClass` "/Game/Mordhau/Maps/Endless/CreatorsStuff/PlacebleCube.PlacebleCube_C" (`KismetMathLibrary.Conv_VectorToTransform` (`KismetMathLibrary.MakeVector` (+ (* (.x (`KismetMathLibrary.Conv_IntVectorToVector` (`.GridLocation_7_7BF930164DAB3D14FA46AF8DBD59BB7E` (break `/Game/Mordhau/Maps/Endless/CreatorsStuff/BlockInfo` _array_element_2)))) 240.0) 20.0) (+ (* (.y (`KismetMathLibrary.Conv_IntVectorToVector` (`.GridLocation_7_7BF930164DAB3D14FA46AF8DBD59BB7E` (break `/Game/Mordhau/Maps/Endless/CreatorsStuff/BlockInfo` _array_element_2)))) 240.0) 20.0) (+ (* (.z (`KismetMathLibrary.Conv_IntVectorToVector` (`.GridLocation_7_7BF930164DAB3D14FA46AF8DBD59BB7E` (break `/Game/Mordhau/Maps/Endless/CreatorsStuff/BlockInfo` _array_element_2)))) 240.0) 20.0))) "AlwaysSpawn" "OverrideRootScale" null _array_element_2 null))
    (set `self.beasy` false)))

(event `ChangeRules`
  (params (NewHealth :type Integer) (NewStamina :type Integer) (HealthRegen :type Boolean :default true) (`AFK kick` :type Boolean))
  (set `self.HealthOnKill` NewHealth)
  (set `self.StaminaOnKill` NewStamina)
  (set `self.bAllowHealthRegen` HealthRegen)
  (set `self.AFKKick` `AFK kick`))

(event `ServerRemoveCube`
  (params (Hit :type "Actor Object Reference"))
  (if (not (`self.beasy`))
    (set `self.beasy` true)
    (bind _asplaceble_cube (cast `/Game/Mordhau/Maps/Endless/CreatorsStuff/PlacebleCube` Hit)
      (:`then`
        (`KismetArrayLibrary.Array_RemoveItem` (`self.CubeGrid`) (`/Game/Mordhau/Maps/Endless/CreatorsStuff/PlacebleCube.BlockInfo` _asplaceble_cube))
        (`self.K2_DestroyActor` Hit))
      (:`CastFailed`
        _))
    (set `self.beasy` false)))

(event `ServerPlaceCube`
  (params (Transform :type "Transform Structure") (BlockInfo :type "/Game/Mordhau/Maps/Endless/CreatorsStuff/BlockInfo Structure"))
  (bind _cubegrid (`self.CubeGrid`))
  (bind (_x _y _z) (break `IntVector` (`.GridLocation_7_7BF930164DAB3D14FA46AF8DBD59BB7E` (break `/Game/Mordhau/Maps/Endless/CreatorsStuff/BlockInfo` BlockInfo))))
  (if (not (`self.beasy`))
    (set `self.beasy` true)
    (for _array_element _cubegrid
      (bind (_x_2 _y_2 _z_2) (break `IntVector` (`.GridLocation_7_7BF930164DAB3D14FA46AF8DBD59BB7E` (break `/Game/Mordhau/Maps/Endless/CreatorsStuff/BlockInfo` _array_element))))
      (if (and (== _x_2 _x) (== _y_2 _y) (== _z_2 _z))
        (bind _output_get (set `self.Has` true))))
    (if (not _output_get)
      (`|SpawnActorFromClass` "/Game/Mordhau/Maps/Endless/CreatorsStuff/PlacebleCube.PlacebleCube_C" Transform "AlwaysSpawn" "OverrideRootScale" null BlockInfo null)
      (`KismetArrayLibrary.Array_Add` _cubegrid BlockInfo))
    (set `self.beasy` false)
    (set `self.Has` false)))

(event `self.ReceiveBeginPlay`
  (bind _returnvalue (`MordhauUtilityLibrary.GetCustomConfigVar_Int` "Endless" "KillsToEndMap" true))
  (bind _returnvalue_2 (`MordhauUtilityLibrary.GetCustomConfigVar_Bool` "Endless" "DisableMenuOptions" true))
  (`parent.ReceiveBeginPlay`)
  (set `self.bAllowSpawning` true)
  (set `self.PostMatchScreenDelay` 0.0)
  (set `self.DefaultEndMatchMapChangeTime` 10.0)
  (set `self.MatchDurationMax` 9999999)
  (set `self.NoScoreInScoreboard` false)
  (set `self.DefaultWarmupTime` 0.0)
  (set `self.EndlessTime` (`KismetMathLibrary.MakeTimespan2` 999 23 59 59))
  (`/Engine/EditorBlueprintResources/ActorMacros.Switch Has Authority`
    (:`Authority`
      (set `self.DisableSettings` _returnvalue_2)
      (set `self.KillsToEndMap` _returnvalue)
      (`MordhauUtilityLibrary.PrintToConsoleAndLog` (`KismetStringLibrary.JoinStringArray` (`|MakeArray` (`KismetStringLibrary.Conv_BoolToString` _returnvalue_2) (`KismetStringLibrary.Conv_IntToString` _returnvalue)) " and ")))))

(event `self.AddKillNotify`
  (params (Killer :type "PlayerState Object Reference") (Killed :type "PlayerState Object Reference") (Weapon :type "Actor Object Reference") (DamageType :type "EMordhauDamageType Enum" :default "Generic"))
  (bind _killstoendmap (`self.KillsToEndMap`))
  (if (== Killer Killed)
    (bind _asbp_mordhau_player_state (cast `/Game/Mordhau/Blueprints/BP_MordhauPlayerState` Killed))
    (`MordhauPlayerState.AddDeaths` _asbp_mordhau_player_state -1)
    (`MordhauPlayerState.AddScore` _asbp_mordhau_player_state 100)
    (else
      (bind _asbp_mordhau_player_state_2 (cast `/Game/Mordhau/Blueprints/BP_MordhauPlayerState` Killer))
      (if (and (>= (`MordhauPlayerState.Kills` _asbp_mordhau_player_state_2) _killstoendmap) (> _killstoendmap 0))
        (bind _asbp_elgame_mode (cast `/Game/Mordhau/Maps/Endless/GameModeBlueprints/BP_ELGameMode` (`GameplayStatics.GetGameMode`)))
        (`GameMode.EndMatch` _asbp_elgame_mode))
      (`parent.AddKillNotify` Killer Killed Weapon DamageType))))

(event `RequestSound`
  (params (NewParam :type "Transform Structure"))
  (`self.ReplicateSound` NewParam))

(event `ReplicateSound`
  (params (NewParam :type "Transform Structure"))
  (`GameplayStatics.SpawnSoundAtLocation` "/Game/Mordhau/Maps/Endless/Assets/Sound/Teleport1.Teleport1" (.location NewParam) (struct) 1.0 1.0 0.0 null null))

(fn `GetScoreboardTime`
  (returns (Time :type "Timespan Structure"))
  (return (`self.EndlessTime`)))

(fn `GetScoreboardTimeInProgress`
  (returns (Time :type "Timespan Structure"))
  (return (`self.EndlessTime`)))

(fn `ShouldHideSpawnInfoText`
  (returns (Hide :type Boolean))
  (return true))

(fn `UserConstructionScript`
  (`parent.UserConstructionScript`))
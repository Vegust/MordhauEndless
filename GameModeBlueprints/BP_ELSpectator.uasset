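; Free-flying spectator pawn with an optional creator mode for placing and removing cubes and switching their color and type.
; Key inputs forward to BP_ELController; holding place or remove repeats via a delayed gate and looping timer, using pawn location and camera rotation.
; Mouse wheel scales flying speed, and collision is disabled outside the Endless level.
; BeginPlay adds the creator widget; unpossession removes it and reports the pawn's location to the controller.
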(event `Key|F`
  (params (Key :type "Key Structure"))
  (:`Pressed`
    (if (not (`self.IsCreator`))
      (bind _asbp_elcontroller (cast `/Game/Mordhau/Maps/Endless/GameModeBlueprints/BP_ELController` (`self.GetController`)))
      (`/Game/Mordhau/Maps/Endless/GameModeBlueprints/BP_ELController.ToggleSnapping` _asbp_elcontroller))))

(event `Key|MouseScrollUp`
  (params (Key :type "Key Structure"))
  (:`Pressed`
    (bind _newspeedmultiplier (`self.ChangeFlyingSpeed` true))
    (bind _asbp_elcontroller (cast `/Game/Mordhau/Maps/Endless/GameModeBlueprints/BP_ELController` (`self.GetController`)))
    (`/Game/Mordhau/Maps/Endless/GameModeBlueprints/BP_ELController.FlyingSpeedChanged` _asbp_elcontroller _newspeedmultiplier)))

(event `Key|MouseScrollDown`
  (params (Key :type "Key Structure"))
  (:`Pressed`
    (bind _newspeedmultiplier (`self.ChangeFlyingSpeed` false))
    (bind _asbp_elcontroller (cast `/Game/Mordhau/Maps/Endless/GameModeBlueprints/BP_ELController` (`self.GetController`)))
    (`/Game/Mordhau/Maps/Endless/GameModeBlueprints/BP_ELController.FlyingSpeedChanged` _asbp_elcontroller _newspeedmultiplier)))

(event `Key|F7`
  (params (Key :type "Key Structure"))
  (:`Pressed`
    (bind _asbp_elcontroller (cast `/Game/Mordhau/Maps/Endless/GameModeBlueprints/BP_ELController` (`self.GetController`)))
    (`/Game/Mordhau/Maps/Endless/GameModeBlueprints/BP_ELController.ShowInfoScreen` _asbp_elcontroller)))

(event `Key|R`
  (params (Key :type "Key Structure"))
  (:`Pressed`
    (`self.TPToZeros`)))

(event `self.ReceiveUnpossessed`
  (params (OldController :type "Controller Object Reference"))
  (bind _asbp_elcontroller (cast `/Game/Mordhau/Maps/Endless/GameModeBlueprints/BP_ELController` OldController)
    (:`then`
      (`Widget.RemoveFromParent` (`self.Widget`))
      (`/Game/Mordhau/Maps/Endless/GameModeBlueprints/BP_ELController.InfoFromSpec` _asbp_elcontroller (`self.K2_GetActorLocation`) (`/Game/Mordhau/Maps/Endless/GameModeBlueprints/BP_ELController.SpawnType` _asbp_elcontroller) (`/Game/Mordhau/Maps/Endless/GameModeBlueprints/BP_ELController.SavedSpawnTransform` _asbp_elcontroller)))
    (:`CastFailed`
      _))
  (`parent.ReceiveUnpossessed` OldController))

(event `SetIsCreator`
  (params (NewValue :type Boolean))
  (bind _output_get (set `self.IsCreator` NewValue))
  (set `/Game/Mordhau/Maps/Endless/GameLogic/CreatorWidget.CreatorStateOpacity` (select `bool` _output_get :`true` 1.0 :!type "Float (single-precision)") (`self.Widget`))
  (bind _asbp_elcontroller (cast `/Game/Mordhau/Maps/Endless/GameModeBlueprints/BP_ELController` (`self.GetController`)))
  (`/Game/Mordhau/Maps/Endless/GameModeBlueprints/BP_ELController.AdjustPreviewToMode` _asbp_elcontroller _output_get))

(event `Key|One`
  (params (Key :type "Key Structure"))
  (:`Pressed`
    (`|ExecutionSequence`
      (:`then_0`
        (goto _label :!via `Open`))
      (:`then_1`
        (`self.PlaceCube`)
        (`KismetSystemLibrary.Delay` 0.2)
        (`/Engine/EditorBlueprintResources/StandardMacros.Gate` true :!label _label
          (:`Exit`
            (bind _returnvalue (`KismetSystemLibrary.K2_SetTimerDelegate` (delegate `PlaceCube`) 0.1 true))
            (set `self.TimerHandle` _returnvalue))))))
  (:`Released`
    (`|ExecutionSequence`
      (:`then_0`
        (goto _label :!via `Close`))
      (:`then_1`
        (`KismetSystemLibrary.K2_ClearAndInvalidateTimerHandle` (`self.TimerHandle`))))))

(event `PlaceCube`
  (if (`self.IsCreator`)
    (bind _asbp_elcontroller (cast `/Game/Mordhau/Maps/Endless/GameModeBlueprints/BP_ELController` (`self.GetController`)))
    (`/Game/Mordhau/Maps/Endless/GameModeBlueprints/BP_ELController.PlaceCube` _asbp_elcontroller (`KismetMathLibrary.MakeTransform` (`self.K2_GetActorLocation`) (`PlayerCameraManager.GetCameraRotation` (`PlayerController.PlayerCameraManager` _asbp_elcontroller))))))

(event `Key|Two`
  (params (Key :type "Key Structure"))
  (:`Pressed`
    (`|ExecutionSequence`
      (:`then_0`
        (goto _label_2 :!via `Open`))
      (:`then_1`
        (`self.RemoveCube`)
        (`KismetSystemLibrary.Delay` 0.2)
        (`/Engine/EditorBlueprintResources/StandardMacros.Gate` true :!label _label_2
          (:`Exit`
            (bind _returnvalue (`KismetSystemLibrary.K2_SetTimerDelegate` (delegate `RemoveCube`) 0.1 true))
            (set `self.TimerHandleR` _returnvalue))))))
  (:`Released`
    (`|ExecutionSequence`
      (:`then_0`
        (goto _label_2 :!via `Close`))
      (:`then_1`
        (`KismetSystemLibrary.K2_ClearAndInvalidateTimerHandle` (`self.TimerHandleR`))))))

(event `RemoveCube`
  (if (`self.IsCreator`)
    (bind _asbp_elcontroller (cast `/Game/Mordhau/Maps/Endless/GameModeBlueprints/BP_ELController` (`self.GetController`)))
    (`/Game/Mordhau/Maps/Endless/GameModeBlueprints/BP_ELController.RemoveCube` _asbp_elcontroller (`KismetMathLibrary.MakeTransform` (`self.K2_GetActorLocation`) (`PlayerCameraManager.GetCameraRotation` (`PlayerController.PlayerCameraManager` _asbp_elcontroller))))))

(event `Key|Three`
  (params (Key :type "Key Structure"))
  (:`Pressed`
    (if (`self.IsCreator`)
      (bind _asbp_elcontroller (cast `/Game/Mordhau/Maps/Endless/GameModeBlueprints/BP_ELController` (`self.GetController`)))
      (`/Game/Mordhau/Maps/Endless/GameModeBlueprints/BP_ELController.SwitchColor` _asbp_elcontroller false))))

(event `Key|Four`
  (params (Key :type "Key Structure"))
  (:`Pressed`
    (if (`self.IsCreator`)
      (bind _asbp_elcontroller (cast `/Game/Mordhau/Maps/Endless/GameModeBlueprints/BP_ELController` (`self.GetController`)))
      (`/Game/Mordhau/Maps/Endless/GameModeBlueprints/BP_ELController.SwitchColor` _asbp_elcontroller true))))

(event `RemoveCollision`
  (`PrimitiveComponent.SetCollisionEnabled` (`self.CollisionComponent`) "NoCollision"))

(event `Key|Five`
  (params (Key :type "Key Structure"))
  (:`Pressed`
    (if (`self.IsCreator`)
      (bind _asbp_elcontroller (cast `/Game/Mordhau/Maps/Endless/GameModeBlueprints/BP_ELController` (`self.GetController`)))
      (`/Game/Mordhau/Maps/Endless/GameModeBlueprints/BP_ELController.SwitchType` _asbp_elcontroller false))))

(event `Key|Six`
  (params (Key :type "Key Structure"))
  (:`Pressed`
    (if (`self.IsCreator`)
      (bind _asbp_elcontroller (cast `/Game/Mordhau/Maps/Endless/GameModeBlueprints/BP_ELController` (`self.GetController`)))
      (`/Game/Mordhau/Maps/Endless/GameModeBlueprints/BP_ELController.SwitchTypeSpecific` _asbp_elcontroller false))))

(event `self.ReceiveBeginPlay`
  (`parent.ReceiveBeginPlay`)
  (`|ExecutionSequence`
    (:`then_0`
      (bind _asfloating_pawn_movement (cast `FloatingPawnMovement` (`self.MovementComponent`)))
      (set `FloatingPawnMovement.Deceleration` 10000000.0 _asfloating_pawn_movement)
      (set `FloatingPawnMovement.Acceleration` 10000000.0 _asfloating_pawn_movement)
      (set `self.StandartFlyingSpeed` (`MovementComponent.GetMaxSpeed` _asfloating_pawn_movement))
      (bind _returnvalue (`GameplayStatics.GetCurrentLevelName` true))
      (if (not (`KismetStringLibrary.EqualEqual_StrStr` _returnvalue "Endless"))
        (`PrimitiveComponent.SetCollisionEnabled` (`self.CollisionComponent`) "NoCollision")))
    (:`then_1`
      (set `self.BlockInputAfterDeathTime` 0.1)
      (`KismetSystemLibrary.Delay` 0.1)
      (`self.SwitchToFreeCam`)
      (bind _asbp_elcontroller (cast `/Game/Mordhau/Maps/Endless/GameModeBlueprints/BP_ELController` (`self.GetController`)))
      (bind _returnvalue_2 (`|CreateWidget` "/Game/Mordhau/Maps/Endless/GameLogic/CreatorWidget.CreatorWidget_C" _asbp_elcontroller))
      (bind _output_get (set `self.Widget` _returnvalue_2))
      (`UserWidget.AddToViewport` _output_get 0)
      (`/Game/Mordhau/Maps/Endless/GameModeBlueprints/BP_ELController.GotSpectatorPawn` _asbp_elcontroller))))

(fn `ChangeFlyingSpeed`
  (params (IsIncreasing :type Boolean))
  (returns (NewSpeedMultiplier :type "Float (double-precision)"))
  (bind _speedmodifier (`self.SpeedModifier`))
  (set `self.SpeedModifier` (select `bool` IsIncreasing :`false` (* _speedmodifier 0.7) :`true` (* _speedmodifier 1.4)))
  (set `self.SpeedModifier` (`KismetMathLibrary.FClamp` _speedmodifier 0.1 9.9))
  (bind _asfloating_pawn_movement (cast `FloatingPawnMovement` (`self.MovementComponent`)))
  (set `FloatingPawnMovement.MaxSpeed` (* _speedmodifier (`self.StandartFlyingSpeed`)) _asfloating_pawn_movement)
  (return _speedmodifier))

(fn `TPToZeros`
  (`self.K2_SetActorTransform` (`KismetMathLibrary.MakeTransform` (0.0 0.0 0.0)) false true))

(fn `UserConstructionScript`
  (`parent.UserConstructionScript`))
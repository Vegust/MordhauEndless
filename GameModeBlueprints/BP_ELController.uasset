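; Player controller for the EL (Endless) Mordhau mode, handling spectator-driven respawns and grid block building.
; Spectator location and camera rotation feed pawn teleports by spawn type (free, ground-snapped, aimed, saved), with timeline-faded warning and timer widgets.
; Creators get a timer-updated preview cube from grid-aligned aim traces.
; Block edits, local save slots and rule changes route through BP_ELGameState; creator and match-end requests through BP_ELGameMode.
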(event `LoadCubes`
  (params (LoadName :type String))
  (bind _returnvalue (`KismetStringLibrary.JoinStringArray` (`|MakeArray` "Endless/" LoadName)))
  ;[1 1 1] Loading
  (bind _returnvalue_2 (`GameplayStatics.DoesSaveGameExist` _returnvalue))
  (if _returnvalue_2
    (bind _returnvalue_3 (`GameplayStatics.LoadGameFromSlot` _returnvalue))
    (bind _asblock_grid_save (cast `/Game/Mordhau/Maps/Endless/CreatorsStuff/BlockGridSave` _returnvalue_3))
    (`self.RequestAppend` (`/Game/Mordhau/Maps/Endless/CreatorsStuff/BlockGridSave.BlockGridInfo` _asblock_grid_save))))

(event `RequestAppend`
  (params (Block :type "Array of /Game/Mordhau/Maps/Endless/CreatorsStuff/BlockInfo Structure"))
  ;[1 1 1] Loading
  (bind _asbp_elgame_state (cast `/Game/Mordhau/Maps/Endless/GameModeBlueprints/BP_ELGameState` (`GameplayStatics.GetGameState`)))
  (`/Game/Mordhau/Maps/Endless/GameModeBlueprints/BP_ELGameState.ServerLoadSaveFile` _asbp_elgame_state Block))

(event `self.OnAFKTimeExceededMaximum`
  (bind _asbp_elgame_state (cast `/Game/Mordhau/Maps/Endless/GameModeBlueprints/BP_ELGameState` (`GameplayStatics.GetGameState`)))
  (if (`/Game/Mordhau/Maps/Endless/GameModeBlueprints/BP_ELGameState.AFKKick` _asbp_elgame_state)
    (`self.PerformAFKKick`)
    (else
      (set `self.CurrentAFKTime` 0.0))))

(event `GetBlockInfo`
  (params (BlockCount :type Integer))
  (set `self.BlockCount` BlockCount))

(event `RequestNumberOfCubes`
  (bind _asbp_elgame_state (cast `/Game/Mordhau/Maps/Endless/GameModeBlueprints/BP_ELGameState` (`GameplayStatics.GetGameState`)))
  (`/Game/Mordhau/Maps/Endless/GameModeBlueprints/BP_ELGameState.ServerInitiateBlockInfoSend` _asbp_elgame_state self))

(event `ChangeRules`
  (params (HP :type Integer) (Stam :type Integer) (HealthRegen :type Boolean) (AFKKick :type Boolean))
  (bind _asbp_elgame_state (cast `/Game/Mordhau/Maps/Endless/GameModeBlueprints/BP_ELGameState` (`GameplayStatics.GetGameState`)))
  (`/Game/Mordhau/Maps/Endless/GameModeBlueprints/BP_ELGameState.ChangeRules` _asbp_elgame_state HP Stam HealthRegen AFKKick))

(event `SaveGame`
  (params (CubeGrid :type "Array of /Game/Mordhau/Maps/Endless/CreatorsStuff/BlockInfo Structure") (SaveName :type String))
  (bind _returnvalue (`GameplayStatics.DoesSaveGameExist` SaveName))
  (if _returnvalue
    (`GameplayStatics.DeleteGameInSlot` SaveName))
  (bind _returnvalue_2 (`GameplayStatics.CreateSaveGameObject` "/Game/Mordhau/Maps/Endless/CreatorsStuff/BlockGridSave.BlockGridSave_C"))
  (set `/Game/Mordhau/Maps/Endless/CreatorsStuff/BlockGridSave.BlockGridInfo` CubeGrid _returnvalue_2)
  (`GameplayStatics.SaveGameToSlot` _returnvalue_2 SaveName))

(event `RequestSaveInfo`
  (params (SaveName :type String))
  (bind _asbp_elgame_state (cast `/Game/Mordhau/Maps/Endless/GameModeBlueprints/BP_ELGameState` (`GameplayStatics.GetGameState`)))
  (`/Game/Mordhau/Maps/Endless/GameModeBlueprints/BP_ELGameState.ServerInniciateSaveOnClient` _asbp_elgame_state self (`KismetStringLibrary.JoinStringArray` (`|MakeArray` "Endless/" SaveName))))

(event `SaveCubes`
  (params (SaveName :type String))
  (`self.RequestSaveInfo` SaveName))

(event `RequestServerReloadCubes`
  (bind _asbp_elgame_state (cast `/Game/Mordhau/Maps/Endless/GameModeBlueprints/BP_ELGameState` (`GameplayStatics.GetGameState`)))
  (`/Game/Mordhau/Maps/Endless/GameModeBlueprints/BP_ELGameState.ServerReloadGrid` _asbp_elgame_state))

(event `ReloadCubes`
  (`self.RequestServerReloadCubes`))

(event `RequestServerClearCubes`
  (bind _asbp_elgame_state (cast `/Game/Mordhau/Maps/Endless/GameModeBlueprints/BP_ELGameState` (`GameplayStatics.GetGameState`)))
  (`/Game/Mordhau/Maps/Endless/GameModeBlueprints/BP_ELGameState.ServerClearGrid` _asbp_elgame_state))

(event `ClearCubes`
  (`self.RequestServerClearCubes`))

(event `RequestServerRemoveCube`
  (params (HitActor :type "Actor Object Reference"))
  (bind _asbp_elgame_state (cast `/Game/Mordhau/Maps/Endless/GameModeBlueprints/BP_ELGameState` (`GameplayStatics.GetGameState`)))
  (`/Game/Mordhau/Maps/Endless/GameModeBlueprints/BP_ELGameState.ServerRemoveCube` _asbp_elgame_state HitActor))

(event `RemoveCube`
  (params (SpecTransform :type "Transform Structure"))
  (bind (_location _hit_actor) (`self.AimLocation` SpecTransform))
  (`self.RequestServerRemoveCube` _hit_actor))

(event `PlaceCube`
  (params (SpecTransform :type "Transform Structure"))
  (bind _location (`self.AimLocation` SpecTransform))
  (bind (_adjustedlocation _gridlocation) (`self.AllignToGrid` _location))
  (`self.RequestServerPlaceCube` (`KismetMathLibrary.MakeTransform` _adjustedlocation) (make `/Game/Mordhau/Maps/Endless/CreatorsStuff/BlockInfo` _gridlocation (`self.ColorNumber`) (`self.TypeNumber`) (`self.TypeSpecific`))))

(event `RequestServerPlaceCube`
  (params (Transform :type "Transform Structure") (BlockInfo :type "/Game/Mordhau/Maps/Endless/CreatorsStuff/BlockInfo Structure"))
  (bind _asbp_elgame_state (cast `/Game/Mordhau/Maps/Endless/GameModeBlueprints/BP_ELGameState` (`GameplayStatics.GetGameState`)))
  (`/Game/Mordhau/Maps/Endless/GameModeBlueprints/BP_ELGameState.ServerPlaceCube` _asbp_elgame_state Transform BlockInfo))

(event `SadFace2`
  (bind _asbp_elgame_mode (cast `/Game/Mordhau/Maps/Endless/GameModeBlueprints/BP_ELGameMode` (`GameplayStatics.GetGameMode`)))
  (`/Game/Mordhau/Maps/Endless/GameModeBlueprints/BP_ELGameMode.RemoveCreator` _asbp_elgame_mode self))

(event `SadFace1`
  (bind _asbp_elgame_mode (cast `/Game/Mordhau/Maps/Endless/GameModeBlueprints/BP_ELGameMode` (`GameplayStatics.GetGameMode`)))
  (`/Game/Mordhau/Maps/Endless/GameModeBlueprints/BP_ELGameMode.NewCreator` _asbp_elgame_mode self))

(event `RequestEndMatch`
  (bind _asbp_elgame_mode (cast `/Game/Mordhau/Maps/Endless/GameModeBlueprints/BP_ELGameMode` (`GameplayStatics.GetGameMode`)))
  (`GameMode.EndMatch` _asbp_elgame_mode))

(event `CorrectPawnPosition`
  (params (Character :type "MordhauCharacter Object Reference") (SpawnType :type Integer))
  (bind _returnvalue (== SpawnType 3))
  (bind _lastspectransform (`self.LastSpecTransform`))
  (switch `int` SpawnType
    (:`0`
      (set `self.SpawnLoc` (.location _lastspectransform)))
    (:`1`
      (bind _location (`self.SnapLocation` _lastspectransform))
      (set `self.SpawnLoc` _location))
    (:`2`
      (bind _location_2 (`self.AimLocation` _lastspectransform))
      (set `self.SpawnLoc` _location_2))
    (:`3`
      (set `self.SpawnLoc` (.location (`self.SavedSpawnTransform`)))))
  (`self.K2_TeleportTo` :`self` Character :`DestLocation` (`self.SpawnLoc`))
  (bind _asbp_elcharacter (cast `/Game/Mordhau/Maps/Endless/GameModeBlueprints/BP_ELCharacter` Character))
  (`/Game/Mordhau/Maps/Endless/GameModeBlueprints/BP_ELCharacter.ReplicatedTurn` _asbp_elcharacter (select `bool` _returnvalue :`false` (.yaw (.rotation _lastspectransform)) :`true` (.yaw (.rotation (`self.SavedSpawnTransform`)))))
  (`/Game/Mordhau/Maps/Endless/GameModeBlueprints/BP_ELCharacter.RepicatedLookUp` _asbp_elcharacter (select `bool` _returnvalue :`false` (.pitch (.rotation _lastspectransform)) :`true` (.pitch (.rotation (`self.SavedSpawnTransform`)))))
  (bind _asbp_elgame_state (cast `/Game/Mordhau/Maps/Endless/GameModeBlueprints/BP_ELGameState` (`GameplayStatics.GetGameState`)))
  (`/Game/Mordhau/Maps/Endless/GameModeBlueprints/BP_ELGameState.RequestSound` _asbp_elgame_state (`KismetMathLibrary.Conv_VectorToTransform` (`self.K2_GetActorLocation` _asbp_elcharacter))))

(event `InfoFromSpec`
  (params (Location :type "Vector Structure") (SpawnType :type Integer) (SavedTransform :type "Transform Structure"))
  (set `self.LastSpecTransform` (`KismetMathLibrary.MakeTransform` Location (`PlayerCameraManager.GetCameraRotation` (`self.PlayerCameraManager`))))
  (set `self.SavedSpawnTransform` SavedTransform)
  (`self.HandleInterfaceRemoval`)
  (bind _asmordhau_character (cast `MordhauCharacter` (`self.K2_GetPawn`)))
  (`self.CorrectPawnPosition` _asmordhau_character SpawnType))

(event `GotSpectatorPawn`
  (bind _warningwidget (`self.WarningWidget`))
  (bind _timewidget (`self.TimeWidget`))
  (bind _timewidget_2 (`self.TimeWidget`))
  (bind _asbp_elplayer_state (cast `/Game/Mordhau/Maps/Endless/GameModeBlueprints/BP_ELPlayerState` (`self.PlayerState`)))
  (set `self.Spectator` (not (== (`MordhauPlayerState.Team` _asbp_elplayer_state) 0)))
  (`|ExecutionSequence`
    (:`then_1`
      (`|ExecutionSequence`
        (:`then_0`
          (`/Engine/EditorBlueprintResources/StandardMacros.DoOnce` false
            (:`Completed`
              (bind _returnvalue (`|CreateWidget` "/Game/Mordhau/Maps/Endless/GameLogic/Warning.Warning_C" self))
              (set `self.WarningWidget` _returnvalue)
              (bind _returnvalue_2 (`|CreateWidget` "/Game/Mordhau/Maps/Endless/GameLogic/RespawnTime.RespawnTime_C" self (`self.SpawnType`)))
              (set `self.TimeWidget` _returnvalue_2))))
        (:`then_1`
          (`UserWidget.AddToViewport` (`self.WarningWidget`) 0)
          (`UserWidget.AddToViewport` (`self.TimeWidget`) 0)
          (`|ExecutionSequence`
            (:`then_0`
              (if (`self.Spectator`)
                (set `/Game/Mordhau/Maps/Endless/GameLogic/RespawnTime.Opacity` 0.0 _timewidget)
                (else
                  (set `/Game/Mordhau/Maps/Endless/GameLogic/RespawnTime.Opacity` 1.0 _timewidget)
                  (bind (_direction _newtrack_0) (`Timeline|Timeline_2` :!via `PlayFromStart` :!label _label)
                    (:`Update`
                      (set `/Game/Mordhau/Maps/Endless/GameLogic/RespawnTime.Time` _newtrack_0 _timewidget_2))
                    (:`Finished`
                      (bind (_direction_2 _newtrack_0_2) (`Timeline|Timeline_3` :!via `PlayFromStart` :!label _label_2)
                        (:`Update`
                          (set `/Game/Mordhau/Maps/Endless/GameLogic/RespawnTime.Opacity` _newtrack_0_2 _timewidget_2))))))))
            (:`then_1`
              (`|ExecutionSequence`
                (:`then_0`
                  (bind (_direction_3 _newtrack_0_3) (`Timeline|Timeline_0` :!via `PlayFromStart` :!label _label_3)
                    (:`Update`
                      (set `/Game/Mordhau/Maps/Endless/GameLogic/Warning.Opacity` _newtrack_0_3 _warningwidget))))
                (:`then_1`
                  (`KismetSystemLibrary.Delay` 3.0)
                  (bind (_direction_4 _newtrack_0_4) (`Timeline|Timeline_1` :!via `PlayFromStart` :!label _label_4)
                    (:`Update`
                      (set `/Game/Mordhau/Maps/Endless/GameLogic/Warning.Opacity` _newtrack_0_4 _warningwidget))))))))))))

(event `HandleInterfaceRemoval`
  (`Widget.RemoveFromParent` (`self.WarningWidget`))
  (`Widget.RemoveFromParent` (`self.TimeWidget`))
  (`|ExecutionSequence`
    (:`then_0`
      (goto _label_3 :!via `Stop`))
    (:`then_1`
      (goto _label_4 :!via `Stop`))
    (:`then_2`
      (goto _label :!via `Stop`))
    (:`then_3`
      (goto _label_2 :!via `Stop`))
    (:`then_4`
      (bind (_direction _newtrack_0) (`Timeline|Timeline_5` :!via `Stop` :!label _label_5)
        (:`Update`
          (set `/Game/Mordhau/Maps/Endless/GameLogic/RespawnTime.Opacity` _newtrack_0 (`self.TimeWidget`)))))
    (:`then_5`
      (goto _label_4 :!via `SetNewTime`))
    (:`then_6`
      (goto _label_2 :!via `SetNewTime`))
    (:`then_7`
      (goto _label_5 :!via `SetNewTime`))))

(event `ToggleSnapping`
  (bind _spawntype (`self.SpawnType`))
  (bind _timewidget (`self.TimeWidget`))
  (if (not (`self.Spectator`))
    (`/Engine/EditorBlueprintResources/StandardMacros.IncrementInt` _spawntype
      (:`  `
        (if (== _spawntype 4)
          (set `self.SpawnType` 0))
        (bind _output_get (set `/Game/Mordhau/Maps/Endless/GameLogic/RespawnTime.SpawnType` (`self.SpawnType`) _timewidget))
        (`|ExecutionSequence`
          (:`then_0`
            (set `/Game/Mordhau/Maps/Endless/GameLogic/RespawnTime.Color` (select `int` _output_get :`0` (1.0 1.0 1.0) :`1` (0.0 1.0 0.0) :`2` (0.2 0.2 1.0) :`3` (1.0 0.0 0.0) :!type "Vector Structure") _timewidget))
          (:`then_1`
            (goto _label_2 :!via `Stop`))
          (:`then_2`
            (goto _label_5 :!via `PlayFromStart`)))))))

(event `FlyingSpeedChanged`
  (params (NewSpeedMultiplier :type "Float (double-precision)"))
  (set `/Game/Mordhau/Maps/Endless/GameLogic/RespawnTime.Speed` NewSpeedMultiplier (`self.TimeWidget`))
  (bind (_direction _newtrack_0) (`Timeline|Timeline_4` :!via `PlayFromStart`)
    (:`Update`
      (set `/Game/Mordhau/Maps/Endless/GameLogic/RespawnTime.SpeedOpacity` _newtrack_0 (`self.TimeWidget`)))))

(event `GetServerAuthorityForSpawn`
  (params (Transform :type "Transform Structure"))
  (message `/Game/Mordhau/Maps/Endless/GameLogic/TPinterface.RequestTP` (`GameplayStatics.GetGameMode`) self Transform))

(event `DebugSound`
  (params (NewParam :type "Transform Structure"))
  (bind _asbp_elgame_state (cast `/Game/Mordhau/Maps/Endless/GameModeBlueprints/BP_ELGameState` (`GameplayStatics.GetGameState`)))
  (`/Game/Mordhau/Maps/Endless/GameModeBlueprints/BP_ELGameState.RequestSound` _asbp_elgame_state NewParam))

(fn `AdjustPreviewToMode`
  (params (IsCreator :type Boolean))
  (if IsCreator
    (bind _location (`self.AimLocation` (`KismetMathLibrary.MakeTransform` (`self.K2_GetActorLocation` (`self.GetSpectatorPawn`)) (`PlayerCameraManager.GetCameraRotation` (`self.PlayerCameraManager`)))))
    (bind (_adjustedlocation _gridlocation) (`self.AllignToGrid` _location))
    (bind _returnvalue (`|SpawnActorFromClass` "/Game/Mordhau/Maps/Endless/CreatorsStuff/PreviewCube.PreviewCube_C" (`KismetMathLibrary.Conv_VectorToTransform` _adjustedlocation) "AlwaysSpawn" "OverrideRootScale" null (make `/Game/Mordhau/Maps/Endless/CreatorsStuff/BlockInfo` _gridlocation (`self.ColorNumber`) (`self.TypeNumber`) (`self.TypeSpecific`)) null))
    (set `self.PreviewCube` _returnvalue)
    (bind _returnvalue_2 (`KismetSystemLibrary.K2_SetTimer` null "MoveCube" 0.01 true))
    (set `self.PreviewHandle` _returnvalue_2)
    (else
      (`self.K2_DestroyActor` (`self.PreviewCube`))
      (`KismetSystemLibrary.K2_ClearAndInvalidateTimerHandle` (`self.PreviewHandle`)))))

(fn `AimLocation`
  (params (Transfrom :type "Transform Structure"))
  (returns (Location :type "Vector Structure") (`Hit Actor` :type "Actor Object Reference"))
  (bind _location (.location Transfrom))
  (bind (_outhit _returnvalue) (`KismetSystemLibrary.LineTraceSingleForObjects` _location (+ _location (`KismetMathLibrary.GreaterGreater_VectorRotator` (100000.0 0.0 0.0) (.rotation Transfrom))) (`|MakeArray` "ObjectTypeQuery1" "ObjectTypeQuery2" :!type "EObjectTypeQuery Enum") false (`|MakeArray` null :!type "Actor Object Reference")))
  (if _returnvalue
    (bind (_bblockinghit _binitialoverlap _time _distance _location_2 _impactpoint _normal _impactnormal _physmat _hitactor _hitcomponent _hitbonename _hititem _faceindex _tracestart _traceend) (`GameplayStatics.BreakHitResult` _outhit))
    (return (+ _impactpoint (* _impactnormal 120.0)) _hitactor)
    (else
      (return (+ (/ (- _traceend _tracestart) 200.0) _location) null))))

(fn `AllignToGrid`
  (params (Location :type "Vector Structure"))
  (returns (AdjustedLocation :type "Vector Structure") (GridLocation :type "IntVector Structure"))
  (bind _returnvalue (`KismetMathLibrary.Round` (/ (+ (.z Location) -20.0) 240.0)))
  (bind _returnvalue_2 (`KismetMathLibrary.Round` (/ (+ (.x Location) -20.0) 240.0)))
  (bind _returnvalue_3 (`KismetMathLibrary.Round` (/ (+ (.y Location) -20.0) 240.0)))
  (return (`KismetMathLibrary.MakeVector` (+ (* _returnvalue_2 240.0) 20.0) (+ (* _returnvalue_3 240.0) 20.0) (+ (* _returnvalue 240.0) 20.0)) (make `IntVector` _returnvalue_2 _returnvalue_3 _returnvalue)))

(fn `CutBlockGridArray`
  (params (BlockGrid :type "Array of /Game/Mordhau/Maps/Endless/CreatorsStuff/BlockInfo Structure")))

(fn `MoveCube`
  (bind _previewcube (`self.PreviewCube`))
  (bind _location (`self.AimLocation` (`KismetMathLibrary.MakeTransform` (`self.K2_GetActorLocation` (`self.GetSpectatorPawn`)) (`PlayerCameraManager.GetCameraRotation` (`self.PlayerCameraManager`)))))
  (bind _adjustedlocation (`self.AllignToGrid` _location))
  (`self.K2_SetActorTransform` _previewcube (`KismetMathLibrary.MakeTransform` _adjustedlocation (struct) (1.05 1.05 1.05)) false true)
  (`/Game/Mordhau/Maps/Endless/CreatorsStuff/PreviewCube.Update` _previewcube (`self.ColorNumber`) (`self.TypeNumber`) (`self.TypeSpecific`)))

(fn `ReqestNewSpawn (Deprecated)`
  (if true
    (if true
      _)))

(fn `ShowInfoScreen`
  (`self.RequestNumberOfCubes`)
  (bind _asbp_elgame_state (cast `/Game/Mordhau/Maps/Endless/GameModeBlueprints/BP_ELGameState` (`GameplayStatics.GetGameState`)))
  (bind _asbp_elspectator (cast `/Game/Mordhau/Maps/Endless/GameModeBlueprints/BP_ELSpectator` (`self.GetSpectatorPawn`)))
  (bind _returnvalue (`|CreateWidget` "/Game/Mordhau/Maps/Endless/GameLogic/SpectatorMenu.SpectatorMenu_C" self (`|MakeArray` "Contraband" "Grad" "Tourney" "Camp" "ThePit" "Taiga" "Feitoria" "Crossroads" "MountainPeak" "bob" "Duelyard" "NandaParbat" "KnightFall" "Terminal" "ContraLite" "Castello" "RockStand") (`/Game/Mordhau/Maps/Endless/GameModeBlueprints/BP_ELSpectator.IsCreator` _asbp_elspectator) (`/Game/Mordhau/Maps/Endless/GameModeBlueprints/BP_ELGameState.HealthOnKill` _asbp_elgame_state) (`/Game/Mordhau/Maps/Endless/GameModeBlueprints/BP_ELGameState.StaminaOnKill` _asbp_elgame_state) (`MordhauGameState.bAllowHealthRegen` _asbp_elgame_state) (`/Game/Mordhau/Maps/Endless/GameModeBlueprints/BP_ELGameState.AFKKick` _asbp_elgame_state)))
  (`WidgetBlueprintLibrary.SetInputMode_UIOnlyEx` self _returnvalue)
  (`UserWidget.AddToViewport` _returnvalue 0)
  (set `self.bShowMouseCursor` true))

(fn `SnapLocation`
  (params (Transform :type "Transform Structure"))
  (returns (Location :type "Vector Structure"))
  (bind _location (.location Transform))
  (bind (_outhit _returnvalue) (`KismetSystemLibrary.LineTraceSingleForObjects` _location (`KismetMathLibrary.MakeVector` (.x _location) (.y _location) (- (.z _location) 100000.0)) (`|MakeArray` "ObjectTypeQuery1" :!type "EObjectTypeQuery Enum")))
  (if _returnvalue
    (return (`KismetMathLibrary.MakeVector` (.x (`.ImpactPoint` (`GameplayStatics.BreakHitResult` _outhit))) (.y (`.ImpactPoint` (`GameplayStatics.BreakHitResult` _outhit))) (+ (.z (`.ImpactPoint` (`GameplayStatics.BreakHitResult` _outhit))) 50.0)))
    (else
      (return _location))))

(fn `SwitchColor`
  (params (Decrease :type Boolean))
  (bind _colornumber (`self.ColorNumber`))
  (if Decrease
    (`/Engine/EditorBlueprintResources/StandardMacros.DecrementInt` _colornumber
      (:`  `
        _))
    (else
      (`/Engine/EditorBlueprintResources/StandardMacros.IncrementInt` _colornumber
        (:`  `
          _))))
  (if (== _colornumber 9)
    (set `self.ColorNumber` 0)
    (elif (== _colornumber -1)
      (set `self.ColorNumber` 8))))

(fn `SwitchType`
  (params (Decrease :type Boolean))
  (bind _typenumber (`self.TypeNumber`))
  (if Decrease
    (`/Engine/EditorBlueprintResources/StandardMacros.DecrementInt` _typenumber
      (:`  `
        _))
    (else
      (`/Engine/EditorBlueprintResources/StandardMacros.IncrementInt` _typenumber
        (:`  `
          _))))
  (if (== _typenumber 3)
    (set `self.TypeNumber` 0)
    (elif (== _typenumber -1)
      (set `self.TypeNumber` 2))))

(fn `SwitchTypeSpecific`
  (params (Decrease :type Boolean))
  (bind _typespecific (`self.TypeSpecific`))
  (if Decrease
    (`/Engine/EditorBlueprintResources/StandardMacros.DecrementInt` _typespecific)
    (else
      (`/Engine/EditorBlueprintResources/StandardMacros.IncrementInt` _typespecific))))

(fn `UserConstructionScript`
  (`parent.UserConstructionScript`))
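; Game mode for a Mordhau "EL" mode with creators: players tracked in CurrentCreators cannot respawn, and the match never ends by itself.
; Shortly after BeginPlay it replaces all player starts with one elevated start and shortens respawn time.
; AddBots doubles as an admin hook, where a magic amount ends the match.
; A deprecated teleport path spawns, equips and possesses a new character at a requested transform.
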(event `RemoveCreator`
  (params (Player :type "PlayerController Object Reference"))
  (`KismetArrayLibrary.Array_RemoveItem` (`self.CurrentCreators`) Player))

(event `NewCreator`
  (params (Player :type "PlayerController Object Reference"))
  (`KismetArrayLibrary.Array_Add` (`self.CurrentCreators`) Player))

(event `self.ReceiveBeginPlay`
  (`parent.ReceiveBeginPlay`)
  (`KismetSystemLibrary.Delay` 0.05)
  (bind _outactors (`GameplayStatics.GetAllActorsOfClass` "/Game/Mordhau/Blueprints/BP_MordhauPlayerStart.BP_MordhauPlayerStart_C"))
  (for _array_element _outactors
    (`self.K2_DestroyActor` _array_element))
  (bind _outactors_2 (`GameplayStatics.GetAllActorsOfClass` "/Script/Mordhau.MordhauPlayerStart"))
  (for _array_element_2 _outactors_2
    (`self.K2_DestroyActor` _array_element_2))
  (`|SpawnActorFromClass` "/Game/Mordhau/Blueprints/BP_MordhauPlayerStart.BP_MordhauPlayerStart_C" (`KismetMathLibrary.MakeTransform` (0.0 0.0 2000.0)) "AdjustIfPossibleButAlwaysSpawn" "OverrideRootScale" null null)
  (set `self.PlayerRespawnTime` 1.0)
  (set `self.bSuicideDecrementsKills` false))

(event `self.AddBots`
  (params (Amount :type Integer) (Team :type Integer))
  (if (== Amount 77)
    (`self.EndMatch`)
    (else
      (`parent.AddBots` Amount Team))))

(event `self.OnScoreChanged`
  (params (State :type "PlayerState Object Reference") (OldValue :type "Float (single-precision)")))

(event `/Game/Mordhau/Maps/Endless/GameLogic/TPinterface.RequestTP`
  (params (Player :type "/Game/Mordhau/Maps/Endless/GameModeBlueprints/BP_ELController Object Reference") (Transform :type "Transform Structure"))
  ;[1 1 1] Deprecated
  (`MordhauPlayerController.ServerRequestSetTeam` Player 0)
  (bind _asbp_elgame_state (cast `/Game/Mordhau/Maps/Endless/GameModeBlueprints/BP_ELGameState` (`GameplayStatics.GetGameState`)))
  (`/Game/Mordhau/Maps/Endless/GameModeBlueprints/BP_ELGameState.RequestSound` _asbp_elgame_state Transform)
  (bind (_body _lookupval) (`self.SpawnBody (Deprecated)` Player Transform))
  (`/Game/Mordhau/Maps/Endless/GameModeBlueprints/BP_ELCharacter.RepicatedLookUp` _body _lookupval)
  (`Controller.Possess` Player _body)
  (bind _asbp_elplayer_state (cast `/Game/Mordhau/Maps/Endless/GameModeBlueprints/BP_ELPlayerState` (`Pawn.PlayerState` _body)))
  (set `MordhauPlayerState.LastMordhauCharacter` _body _asbp_elplayer_state))

(fn `PlayerCanRestart`
  (params (Player :type "PlayerController Object Reference"))
  (returns (ReturnValue :type Boolean))
  (bind _returnvalue (`parent.PlayerCanRestart` Player))
  (return (and _returnvalue (not (`KismetArrayLibrary.Array_Contains` (`self.CurrentCreators`) Player)))))

(fn `ReadyToEndMatch`
  (returns (ReturnValue :type Boolean))
  (return false))

(fn `SpawnBody (Deprecated)`
  (params (player :type "/Game/Mordhau/Maps/Endless/GameModeBlueprints/BP_ELController Object Reference") (NewParam1 :type "Transform Structure"))
  (returns (body :type "/Game/Mordhau/Maps/Endless/GameModeBlueprints/BP_ELCharacter Object Reference") (lookupval :type "Float (double-precision)"))
  (locals (QuiverSet :type Boolean))
  (bind _pendingcharacterprofile (`MordhauPlayerController.PendingCharacterProfile` player))
  (bind (_name _gearcustomization _appearancecustomization) (break `CharacterProfile` _pendingcharacterprofile))
  (bind _pitch (.pitch (.rotation NewParam1)))
  (bind (_wearables _equipment) (break `CharacterGearCustomization` _gearcustomization))
  (bind (_emblem _emblemcolors) (break `AppearanceCustomization` _appearancecustomization))
  (bind _returnvalue (`|SpawnActorFromClass` "/Game/Mordhau/Maps/Endless/GameModeBlueprints/BP_ELCharacter.BP_ELCharacter_C" (`KismetMathLibrary.MakeTransform` (.location NewParam1) (`KismetMathLibrary.MakeRotator` 0.0 0.0 (.yaw (.rotation NewParam1)))) "Undefined" "OverrideRootScale" null null))
  (for (_ _array_index) _equipment
    (bind _returnvalue_2 (`MordhauSingleton.SpawnEquipment` (`MordhauUtilityLibrary.GetMordhauSingleton`) (`MordhauUtilityLibrary.GetWorldOf` _returnvalue) (`|GetArrayItem` _equipment _array_index) (`KismetMathLibrary.Conv_IntToByte` _emblem) (`|GetArrayItem` _emblemcolors) (`|GetArrayItem` _emblemcolors 1) false false))
    (bind _quiver (`MordhauEquipment.Quiver` _returnvalue_2))
    (if (`KismetSystemLibrary.IsValidClass` _quiver)
      (if (not (`local.QuiverSet`))
        (set `local.QuiverSet` true)
        (`MordhauCharacter.SetQuiver` _returnvalue _quiver)))
    (`MordhauCharacter.PickUp` _returnvalue _returnvalue_2 0))
  (`MordhauCharacter.AssignProfile` _returnvalue _pendingcharacterprofile)
  (set `local.QuiverSet` false)
  (return _returnvalue (select `bool` (< _pitch 270.0) :`false` (+ _pitch -360.0) :`true` _pitch)))

(fn `UserConstructionScript`
  (`parent.UserConstructionScript`))
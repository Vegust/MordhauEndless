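; BP_SpecSphere is a particle-folder actor that shadows another actor referenced by its Spec variable.
; On BeginPlay it sets a fast tick interval, then each tick copies the full transform of Spec onto itself.
; A GotSpec flag latches on the first valid tick, so the sphere waits for Spec to be assigned and destroys itself only once that actor later becomes invalid.
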(event `self.ReceiveBeginPlay`
  (`self.SetActorTickInterval` 0.01))

(event `self.ReceiveTick`
  (params (DeltaSeconds :type "Float (single-precision)"))
  (bind _spec (`self.Spec`))
  (bind _gotspec (`self.GotSpec`))
  (`/Engine/EditorBlueprintResources/StandardMacros.IsValid` _spec
    (:`Is Valid`
      (if _gotspec
        (`self.K2_SetActorTransform` (`self.GetTransform` _spec))
        (else
          (set `self.GotSpec` true))))
    (:`Is Not Valid`
      (if _gotspec
        (`self.K2_DestroyActor`)))))

(fn `UserConstructionScript`)